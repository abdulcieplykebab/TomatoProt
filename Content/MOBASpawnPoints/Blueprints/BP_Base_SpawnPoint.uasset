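; Base wave spawn point for a MOBA-style mode that spawns creep waves on a timer and shows a colored name and next-wave countdown.
; Tick drives the timer, optionally waiting until all tracked creeps are dead, and the authority spawns the creep list with a per-creep delay.
; After its last wave it destroys itself, unless it is the last spawner, which spawns an optional boss or otherwise triggers the game win.
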(event `self.ReceiveBeginPlay`
  ;[0 0 0] Start counting time by default when Play begins.
  (set `self.bEnableTimer` true))

(event `self.ReceiveTick`
  (params (DeltaSeconds :type "Float (single-precision)"))
  ;[0 0 0] Creates and monitors the Spawn Timer for this Spawner.
  (`self.UpdateRespawnTimerText`)
  (if (`self.bEnableTimer`)
    (set `self.TotalElapsedTime` (+ (* DeltaSeconds 1.0) (`self.TotalElapsedTime`)))
    (bind _output_get (set `self.ElapsedTime` (+ (* DeltaSeconds 1.0) (`self.ElapsedTime`))))
    (if (>= _output_get (`self.WaveTimeInSeconds`))
      (set `self.ElapsedTime` 0.0)
      ;;[1 1 1] Kill all to next weave
      (if (`self.KillAllToNextWeave`)
        (if (== (`KismetArrayLibrary.Array_Length` (`self.SpawnedCreeps`)) 0)
          ;;[1 1 1] spawn only defined weave count
          (if (>= (`self.CurrentWaveNumber`) (`self.WeaveCount`)) :!label _label
            ;[1 1 1] dodac bool = bchceszpanbossa?
            (bind _outactors (`GameplayStatics.GetAllActorsOfClass` "BP_Base_SpawnPoint_C"))
            (if (<= (`KismetArrayLibrary.Array_Length` _outactors) 1)
              (if (`self.ChceszBossa`)
                (set `self.bEnableTimer` false)
                (`|SpawnActorFromClass` (`self.BossChar`) (`self.GetTransform` self) "Undefined" "OverrideRootScale" null null)
                (`KismetSystemLibrary.PrintString` "boss spawned")
                (else
                  ;[1 1 1] No Boss & No Spawners == End Game
                  (`self.K2_DestroyActor`)
                  (message `/Game/TwinStickBP/GameMode/IGameMode.WinGame` (`GameplayStatics.GetGameMode`))))
              (else
                ;[1 1 1] Kilim aby urodzic bossa gdy wszystkie spawnery skoncza
                (`self.K2_DestroyActor`)))
            (else
              (set `self.CurrentWaveNumber` (+ (`self.CurrentWaveNumber`) 1))
              (`/Engine/EditorBlueprintResources/ActorMacros.Switch Has Authority`
                (:`Authority`
                  (`/Game/MOBASpawnPoints/Blueprints/IMOBASpawner.SpawnCreepWave`)))))
          (else
            (`KismetSystemLibrary.PrintString` "kill all first")))
        (else
          (goto _label))))
    (else
      (set `self.ElapsedTime` 0.0) ; If the Timer is disabled we need to reset our ElapsedTime
    )))

(event `/Game/MOBASpawnPoints/Blueprints/IMOBASpawner.SpawnCreepWave`
  (bind (_returnvalue_location _returnvalue_rotation) (`KismetMathLibrary.BreakTransform` (`SceneComponent.K2_GetComponentToWorld` (`self.ArrowForwardVector`))))
  ;[0 0 0] Default Spawning Behavior
  (`/Engine/EditorBlueprintResources/ActorMacros.Switch Has Authority`
    (:`Authority`
      (if (== (`KismetArrayLibrary.Array_Length` (`self.CreepsToSpawn`)) 0)
        (if (`self.bEnableDebugMessages`)
          (`KismetSystemLibrary.PrintString` "WARNING: No creeps to spawn from Base Spawner!" true true (struct :`R` 1.0 :`G` 1.0 :`A` 1.0)))
        (else
          (set `self.bEnableTimer` false)
          (bind _array_element (`/Game/MOBASpawnPoints/Blueprints/BP_MOBA_MacroLibrary.ForEachLoopWithDelay` (`self.CreepsToSpawn`) :!label _label_2)
            (:`Loop Body`
              (bind _returnvalue (`|SpawnActorFromClass` _array_element (`KismetMathLibrary.MakeTransform` _returnvalue_location _returnvalue_rotation) "AdjustIfPossibleButAlwaysSpawn" "OverrideRootScale" null null))
              (`KismetArrayLibrary.Array_Add` (`self.SpawnedCreeps`) _returnvalue)
              (`KismetSystemLibrary.Delay` (`self.PerCreepSpawnDelay`))
              (goto _label_2 :!via `Next Iteration`))
            (:`Completed`
              (set `self.bEnableTimer` true))))))))

(event `/Game/MOBASpawnPoints/Blueprints/IMOBASpawner.CreepHasDied`
  (params (Creep :type "Actor Object Reference"))
  (bind _spawnedcreeps (`self.SpawnedCreeps`))
  ;[0 0 0] Default logic for when a Creep dies. Simply removes it from the internal array of Creep references.
  (for (_array_element _array_index) _spawnedcreeps
    (if (== _array_element Creep)
      (`KismetArrayLibrary.Array_Remove` _spawnedcreeps _array_index)
      (break))))

(fn `GetCurrentCreeps`
  (returns (Creeps :type "Array of Actor Object Reference"))
  ;[0 0 0] Returns the currently spawned and alive creeps that came from this Spawner.
  (return (`self.SpawnedCreeps`)))

(fn `GetCurrentWaveNumber`
  (returns (CurrentWaveNumber :type Integer))
  ;[0 0 0] Returns which number wave the Spawner is up to.
  (return (`self.CurrentWaveNumber`)))

(fn `GetNextWaveTime`
  (returns (NextWaveInSeconds :type "Float (double-precision)"))
  ;[0 0 0] Time counts up, so to get our next Spawn Wave time we have to subtract our ElapsedTime from the WaveTimeinSeconds
  (return (- (`self.WaveTimeInSeconds`) (`self.ElapsedTime`))))

(fn `UpdateRespawnTimerText`
  ;[0 0 0] Simply gets the next spawn timer and updates the text for this spawner.
  (bind _nextwaveinseconds (`/Game/MOBASpawnPoints/Blueprints/IMOBASpawner.GetNextWaveTime`))
  (`TextRenderComponent.K2_SetText` (`self.NextWaveTimeTextRender`) (`KismetTextLibrary.Conv_StringToText` (`KismetStringLibrary.BuildString_Int` "Next Wave In: " "" (`KismetMathLibrary.FTrunc` _nextwaveinseconds)))))

(fn `UserConstructionScript`
  (bind _spawnercolor (`self.SpawnerColor`))
  (bind _spawnernametextrender (`self.SpawnerNameTextRender`))
  ;[0 0 0] Build the Spawners Name and setup its colors.
  (`TextRenderComponent.K2_SetText` _spawnernametextrender (`self.SpawnersName`))
  (`TextRenderComponent.SetTextRenderColor` _spawnernametextrender (`KismetMathLibrary.Conv_LinearColorToColor` _spawnercolor))
  (`ArrowComponent.SetArrowColor` (`self.ArrowForwardVector`) _spawnercolor)
  (`TextRenderComponent.SetTextRenderColor` (`self.NextWaveTimeTextRender`) (`KismetMathLibrary.Conv_LinearColorToColor` _spawnercolor)))