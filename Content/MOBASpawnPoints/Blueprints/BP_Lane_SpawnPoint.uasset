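; MOBA lane spawn point that spawns creep waves on the server and tracks live creeps until notified of their death.
; BeginPlay enables the spawn timer; each wave temporarily appends the first matching wave-specific group, chosen by start wave and modulus-based frequency.
; Creeps are optionally grouped by class, then spawned at the arrow with a per-creep delay.
; Spawned creeps receive a reference to the spawner through ISpawnableCreep.
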(event EventSpawnCreepWave
  ;[0 0 0] Adds the specific wave creeps to the Base Creep array before Spawning and then cleans up those that are only spawning at a specific wave.
  (Networking|SwitchHasAuthority
    (:Authority
      (CallFunction|AddAdditionalCreeps) ; Before we Spawn this wave we need to determine if there are any additional Creeps specific to this Wave that have to also be spawned.
      (if (== (Utilities|Array|Length (Variables|Default|GetCreepsToSpawn)) 0)
        (if (Variables|Default|GetbEnableDebugMessages)
          (Development|PrintString "WARNING: No creeps to spawn from Lane Spawner!" true true "(R=1.000000,G=1.000000,B=0.000000,A=1.000000)"))
        (else
          (if (Variables|Spawning|GetbSpawnCreepsInOrder)
            (CallFunction|SortWaveCreepOrder) ; Sort the order of the Creeps before Spawning so that they all appear together.
          )
          (if (Variables|Default|GetbEnableDebugMessages)
            (Development|PrintString "Spawning new Lane Wave!"))
          (bind _array_element (Utilities|ForEachLoopwithDelay (Variables|Default|GetCreepsToSpawn) :!label _label)
            (:Loop%20Body
              (bind _returnvalue (Game|SpawnActorfromClass _array_element (Transformation|GetWorldTransform (Variables|Default|GetArrowForwardVector)) "AdjustIfPossibleButAlwaysSpawn" 0 0))
              (Utilities|Array|Add (Variables|Default|GetSpawnedCreeps) _returnvalue)
              ;;[1 0 0] THIS INTERFACE NEEDS TO BE IMPLEMENTED BY YOUR BASE AI CLASS TYPE
              (if (Utilities|DoesObjectImplementInterface _returnvalue "/Game/MOBASpawnPoints/Blueprints/ISpawnableCreep.ISpawnableCreep_C")
                (Class|ISpawnableCreep|SetSpawnPoint(Message) _returnvalue self)
                (elif (Variables|Default|GetbEnableDebugMessages)
                  (Development|PrintString "WARNING: Spawned Actor does not implement the ISpawnableCreep interface from Lane Spawner!" true true "(R=1.000000,G=1.000000,B=0.000000,A=1.000000)")))
              (Utilities|FlowControl|Delay (Variables|Default|GetPerCreepSpawnDelay))
              (goto _label Next%20Iteration))
            (:Completed
              (CallFunction|RemoveWaveSpecificCreeps) ; Finally we need to remove all Creeps that do not need to Spawn on the next Wave.
            )))))))

(event EventBeginPlay
  ;[0 0 0] Enable our Spawn Timer to begin counting time when Play starts.
  (Variables|Default|SetbEnableTimer true))

(event EventCreepHasDied
  (params (Creep :type Actor%20Object%20Reference))
  (bind _spawnedcreeps (Variables|Default|GetSpawnedCreeps))
  ;[0 0 0] Event to notify this Spawner that a Creep has died and to update its internal array of Creep references.
  (bind (_array_element _array_index) (Utilities|Array|ForEachLoopwithBreak _spawnedcreeps :!label _label)
    (:LoopBody
      (if (== _array_element Creep)
        (Utilities|Array|RemoveIndex _spawnedcreeps _array_index)
        (goto _label Break)))))

(fn ConstructionScript
  (|CallParentFunction))

(fn AddAdditionalCreeps
  (bind _currentwavenumber (Variables|Default|GetCurrentWaveNumber))
  ;[0 0 0] Appends the additional Creeps to the Base Creep Array to allow them to Spawn on this wave.
  (bind _array_element (Utilities|Array|ForEachLoopwithBreak (Variables|Spawning|GetWaveSpecificCreeps) :!label _label)
    (:LoopBody
      (if (== (.wavetobeginspawningat _array_element) _currentwavenumber)
        (Utilities|Array|AppendArray (Variables|Default|GetCreepsToSpawn) (.creeps _array_element) :!label _label_2)
        (goto _label Break)
        (elif (and (Math|Boolean|NotEqual(Boolean) (.bonlyspawnonthiswave _array_element) true) (== (|(((CurrentWave-StartWave)/WaveFreq)%1) (Math|Conversions|ToFloat(Integer) _currentwavenumber) (Math|Conversions|ToFloat(Integer) (.wavetobeginspawningat _array_element)) (Math|Conversions|ToFloat(Integer) (.creepwavefrequency _array_element))) 0.0)) ; If the return from our Math Expression is 0 then we can Spawn on this wave.
          (goto _label_2))))))

(fn SortWaveCreepOrder
  ;[0 0 0] Sorts the Base Creep Array so that the Creeps appear together based on their class type as they spawn.
  (bind _output_get (LocalVariables|SetUnsortedCreeps (Variables|Default|GetCreepsToSpawn)))
  (if (!= (Utilities|Array|Length _output_get) 0) :!label _label
    (for (_array_element _array_index) (LocalVariables|GetUnsortedCreeps)
      (if (== _array_index 0)
        (bind _output_get_2 (LocalVariables|SetCurrentCreepType _array_element)))
      (if (== _output_get_2 _array_element)
        (Utilities|Array|Add (LocalVariables|GetSortedCreeps) _array_element)
        (Utilities|Array|RemoveIndex (LocalVariables|GetUnsortedCreeps) _array_index)))
    (goto _label)
    (else
      (Utilities|Array|Clear (Variables|Default|GetCreepsToSpawn))
      (for _array_element_2 (LocalVariables|GetSortedCreeps)
        (bind _asactor (Utilities|Casting|CastToActorClass _array_element_2))
        (Utilities|Array|Add (Variables|Default|GetCreepsToSpawn) _asactor)))))

(fn RemoveWaveSpecificCreeps
  ;[0 0 0] Removes any Creeps that are marked to Spawn only on a particular Wave.
  (bind _array_element (Utilities|Array|ForEachLoopwithBreak (Variables|Spawning|GetWaveSpecificCreeps) :!label _label)
    (:LoopBody
      (if (and (.bonlyspawnonthiswave _array_element) (== (.wavetobeginspawningat _array_element) (Variables|Default|GetCurrentWaveNumber)))
        (for _array_element_2 (.creeps _array_element) :!label _label_2
          (for (_array_element_3 _array_index) (Variables|Default|GetCreepsToSpawn)
            (if (== _array_element_3 _array_element_2)
              (Utilities|Array|RemoveIndex (Variables|Default|GetCreepsToSpawn) _array_index))))
        (goto _label Break)
        (elif (== (|(((CurrentWave-StartWave)/WaveFreq)%1) (Math|Conversions|ToFloat(Integer) (Variables|Default|GetCurrentWaveNumber)) (Math|Conversions|ToFloat(Integer) (.wavetobeginspawningat _array_element)) (Math|Conversions|ToFloat(Integer) (.creepwavefrequency _array_element))) 0.0) ; If the return from the modulus calculation is not 0, then we need to remove these Creeps from the Wave.
          (goto _label_2))))))